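; Car pawn Blueprint that tracks whether the car is on the ground and flashes it yellow while invincible.
; Each Tick, a visibility line trace from the box component, offset using the actor's up vector, sets IsOnGround.
; CallInvincible plays a timeline that drives the Yellowness parameter on a dynamic material created in the construction script.
; Tick resets Yellowness and stops the timeline whenever Invincible is false.
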(event `self.ReceiveTick`
  (params (DeltaSeconds :type "Float (single-precision)"))
  (bind _carmaterial (`self.CarMaterial`))
  (bind _returnvalue (`SceneComponent.K2_GetComponentLocation` (`self.BoxComponent`)))
  (bind (_outhit _returnvalue_2) (`KismetSystemLibrary.LineTraceSingle` :`Start` _returnvalue :`End` (+ _returnvalue (* (1.0 1.0 -100.0) (`self.GetActorUpVector`))) :`TraceChannel` "TraceTypeQuery1" :`DrawDebugType` "ForOneFrame"))
  (set `self.IsOnGround` _returnvalue_2)
  ;[1 1 1] Flash Yellow and send to Matrial Instance
  (if (not (`self.bInvincible`))
    ;;[1 1 1] Set Yellowness to 0
    (`MaterialInstanceDynamic.SetScalarParameterValue` _carmaterial "Yellowness" 0.0)
    (bind (_direction _newtrack_0) (`Timeline|Timeline_0` :!via `Stop` :!label _label)
      (:`Update`
        (`MaterialInstanceDynamic.SetScalarParameterValue` _carmaterial "Yellowness" _newtrack_0)))))

(event `self.CallInvincible`
  ;[1 1 1] Flash Yellow and send to Matrial Instance
  (goto _label))

(fn `UserConstructionScript`
  ;[1 1 1] Create Material Instance for each block
  (bind _returnvalue (`PrimitiveComponent.CreateDynamicMaterialInstance` (`self.StaticMesh`) 0 null))
  (set `self.CarMaterial` _returnvalue))